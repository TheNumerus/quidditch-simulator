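; Test actor that draws a projectile's parabolic trajectory as a procedural ribbon mesh.
; VypocetX and VypocetZ compute ballistic positions from speed, angle and gravity, with speed and angle optionally derived from a test input vector.
; The construction script builds paired vertices, UVs and alternating-winding triangles, then applies the test material.
; Tick recomputes the vertices and updates the mesh section in place.
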(event EventTick
  (params (DeltaSeconds :type Float%20%28single-precision%29))
  (Utilities|Array|Clear (Variables|Default|GetTestVertices))
  (for _index (range 0 (Variables|Default|GetPocetKroku))
    (Variables|Default|SetCas (/ (Math|Conversions|ToFloat(Integer) _index) (Variables|Default|GetMeritkoCasu)))
    (Utilities|Array|Add (Variables|Default|GetTestVertices) (Math|Vector|MakeVector (Utilities|VypocetX (Variables|Default|GetCas)) -1e+01 (Utilities|VypocetZ (Variables|Default|GetCas))))
    (Utilities|Array|Add (Variables|Default|GetTestVertices) (Math|Vector|MakeVector (Utilities|VypocetX (Variables|Default|GetCas)) 1e+01 (Utilities|VypocetZ (Variables|Default|GetCas)))))
  (Class|ProceduralMeshComponent|UpdateMeshSection (Variables|Default|GetNewVar_0) 0 (Variables|Default|GetTestVertices) 0 (Variables|Default|GetArrayUV)))

(fn ConstructionScript
  (bind _testinput (Variables|Default|GetTestInput))
  (bind _testtris (Variables|Default|GetTestTris))
  (bind _testtris_2 (Variables|Default|GetTestTris))
  (bind (_x _y _z) (Math|Vector|BreakVector _testinput))
  (if (Variables|Default|GetTestInputTrue)
    (Variables|Default|SetSmer (Class|KismetMathLibrary|DegAtan (/ _z _x)))
    (Variables|Default|SetRychlost (Math|Vector|VectorLength _testinput)))
  (for _index (range 0 (Variables|Default|GetPocetKroku))
    (Variables|Default|SetCas (/ (Math|Conversions|ToFloat(Integer) _index) (Variables|Default|GetMeritkoCasu)))
    (Utilities|Array|Add (Variables|Default|GetTestVertices) (Math|Vector|MakeVector (Utilities|VypocetX (Variables|Default|GetCas)) -1e+01 (Utilities|VypocetZ (Variables|Default|GetCas))))
    (Utilities|Array|Add (Variables|Default|GetTestVertices) (Math|Vector|MakeVector (Utilities|VypocetX (Variables|Default|GetCas)) 1e+01 (Utilities|VypocetZ (Variables|Default|GetCas))))
    (Utilities|Array|Add (Variables|Default|GetArrayUV) "(X=0.000000,Y=0.000000)")
    (Utilities|Array|Add (Variables|Default|GetArrayUV) "(X=1.000000,Y=0.000000)"))
  (for _index_2 (range 0 (+ (/ (Utilities|Array|Length (Variables|Default|GetTestVertices)) 3) 1))
    (if (== (Math|Integer|%(Integer) _index_2 2) 0)
      (Utilities|Array|Add _testtris (+ _index_2 0))
      (Utilities|Array|Add _testtris (+ _index_2 1))
      (Utilities|Array|Add _testtris (+ _index_2 2))
      (else
        (Utilities|Array|Add _testtris_2 (+ _index_2 1))
        (Utilities|Array|Add _testtris_2 (+ _index_2 0))
        (Utilities|Array|Add _testtris_2 (+ _index_2 2)))))
  (bind _returnvalue (AddComponent|AddProceduralMeshComponent false))
  (bind _output_get (Variables|Default|SetNewVar_0 _returnvalue))
  (Class|ProceduralMeshComponent|CreateMeshSection _output_get 0 (Variables|Default|GetTestVertices) (Variables|Default|GetTestTris) 0 (Variables|Default|GetArrayUV) 0 0 false)
  (Rendering|Material|SetMaterial _output_get 0 "/Game/PetrovyRandomHovna/M_ParabolaTest.M_ParabolaTest"))
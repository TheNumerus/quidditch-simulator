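; BP_SplineTest is a test Blueprint that draws a parabolic arc from cylinder spline meshes, resembling a trajectory shaped by a Gravity variable.
; Its Construction Script adds spline mesh components in a loop, stepping each evenly along X and offsetting Z by the squared index times Gravity.
; Each segment ends where the next begins; tangents are never set, and the event graph has no active logic.
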(event EventBeginPlay)

(event EventActorBeginOverlap
  (params (OtherActor :type Actor%20Object%20Reference)))

(event EventTick
  (params (DeltaSeconds :type Float%20%28single-precision%29)))

(fn ConstructionScript
  (for _index (range 0 10)
    (bind _returnvalue (AddComponent|AddSplineMeshComponent false))
    (bind _output_get (LocalVariables|SetNewLocalVar_0 _returnvalue))
    (Components|StaticMesh|SetStaticMesh _output_get "/Game/StarterContent/Shapes/Shape_Cylinder.Shape_Cylinder")
    (SplineMesh|SetStartPosition (LocalVariables|GetNewLocalVar_0) (+ (* "100.000000, 0, 0" _index) (Math|Vector|MakeVector 0.0 0.0 (* (* _index _index) (Variables|Default|GetGravity)))))
    (SplineMesh|SetEndPosition (LocalVariables|GetNewLocalVar_0) (+ (* "100.000000, 0, 0" (+ _index 1)) (Math|Vector|MakeVector 0.0 0.0 (* (* (+ _index 1) (+ _index 1)) (Variables|Default|GetGravity)))))))
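; BP_Potlouk is a ball actor (Czech for Bludger) that chases nearby FlyingPawn players.
; Each tick, JsouPoblizHraci sphere-sweeps along world +Y for players; without a target, it randomly picks one, testing line of sight against WorldStatic.
; It moves by swept, delta-time-scaled offsets, slowing near the target and stopping when very close.
; When static geometry blocks the view, it takes one random-direction step and drops the target.
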(event EventTick
  (params (DeltaSeconds :type Float%20%28single-precision%29))
  (bind _returnvalue (Transformation|GetActorLocation))
  (bind _zpomaleniuhrace (Variables|Default|GetZpomaleniUHrace))
  ;[1 1 1] Zacileni
  (bind _hraci (CallFunction|JsouPoblizHraci (Variables|Default|GetRadius)))
  (if (Variables|Default|GetJeCil)
    ;[1 1 1] Pronasledovani Hrace
    (bind _returnvalue_2 (Collision|LineTraceForObjects _returnvalue (Transformation|GetWorldLocation (Variables|/Game/FlyingBP/Blueprints/FlyingPawn.FlyingPawn_C|GetTarget (Variables|Default|GetCil))) (Utilities|Array|MakeArray "ObjectTypeQuery1") false 0 "None" :!label _label))
    (if _returnvalue_2
      (Transformation|AddActorLocalOffset (* (* (Math|Vector|Normalize (Math|Vector|MakeVector (Math|Random|RandomFloatinRange -1.0 1.0) (Math|Random|RandomFloatinRange -1.0 1.0) (Math|Random|RandomFloatinRange -1.0 1.0))) 5e+02) (Utilities|Time|GetWorldDeltaSeconds)) true false)
      (Variables|Default|SetCil 0)
      (Variables|Default|SetJeCil false)
      (elif (not (< (Math|Vector|VectorLength (- (Transformation|GetWorldLocation (Variables|/Game/FlyingBP/Blueprints/FlyingPawn.FlyingPawn_C|GetTarget (Variables|Default|GetCil))) _returnvalue)) 5e+01))
        (Transformation|AddActorLocalOffset (* (* (Math|Vector|Normalize (- (Transformation|GetWorldLocation (Variables|/Game/FlyingBP/Blueprints/FlyingPawn.FlyingPawn_C|GetTarget (Variables|Default|GetCil))) _returnvalue)) (* (/ (Math|Float|Clamp(Float) (Math|Vector|VectorLength (- (Transformation|GetWorldLocation (Variables|/Game/FlyingBP/Blueprints/FlyingPawn.FlyingPawn_C|GetTarget (Variables|Default|GetCil))) _returnvalue)) 0.0 _zpomaleniuhrace) _zpomaleniuhrace) (Variables|Default|GetRychlost))) (Utilities|Time|GetWorldDeltaSeconds)) true false) ; Posun, kdyz najde hrace
      ))
    (elif (not (== (- (Utilities|Array|Length _hraci) 1) -1)) ; Kdyz je pole hracu prazdne, nedeje se nic
      (bind _returnvalue_3 (Collision|LineTraceForObjects (Transformation|GetActorLocation) (Transformation|GetWorldLocation (Variables|/Game/FlyingBP/Blueprints/FlyingPawn.FlyingPawn_C|GetTarget (Utilities|Array|Get(acopy) _hraci (Math|Random|RandomIntegerinRange 0 (- (Utilities|Array|Length _hraci) 1))))) (Utilities|Array|MakeArray "ObjectTypeQuery1") false 0 "None"))
      (if (not _returnvalue_3)
        (Variables|Default|SetCil (Utilities|Array|Get(acopy) _hraci (Math|Random|RandomIntegerinRange 0 (- (Utilities|Array|Length _hraci) 1))))
        (Variables|Default|SetJeCil true)
        (goto _label)))))

(fn ConstructionScript)

(fn JsouPoblizHraci
  (params (Radius :type Float%20%28single-precision%29))
  (bind _returnvalue (Transformation|GetActorLocation))
  (bind _outhits (Collision|MultiSphereTraceForObjects _returnvalue (+ _returnvalue "0,800.000000, 0") Radius (Utilities|Array|MakeArray "ObjectTypeQuery2") true 0 "None" false))
  (for _array_element _outhits
    (bind _asflying_pawn (Utilities|Casting|CastToFlyingPawn (.HitActor (Collision|BreakHitResult _array_element))))
    (Utilities|Array|Add (LocalVariables|GetPoleHracu) _asflying_pawn))
  (return (LocalVariables|GetPoleHracu)))